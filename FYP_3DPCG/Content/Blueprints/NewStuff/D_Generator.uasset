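; D_Generator procedurally builds a level at BeginPlay by chaining randomly picked rooms from RoomList, starting from a DRoom1 at its own transform.
; Each room spawns at a random open exit; after a short delay its overlap boxes are checked, and an overlapping room is destroyed and retried.
; Accepted rooms add their exits to the pool until RoomCount runs out, then ExitWall actors seal the remaining exits.
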(event Custom|SpawnStartRoom
  ;[0.15 0.15 0.15 0.5 25] Spawn the starting room
  (bind _returnvalue (Game|SpawnActorfromClass "/Game/Blueprints/NewStuff/DRoom1.DRoom1_C" (Transformation|GetWorldTransform (Variables|Default|GetDefaultSceneRoot)) "AlwaysSpawn" "MultiplyWithRoot" 0 0))
  (Utilities|Array|AppendArray (Variables|Default|GetExitsList) (Components|GetChildrenComponents (Variables|/Game/Blueprints/NewStuff/Master_Room.Master_Room_C|GetExitsFolder _returnvalue) false)))

(event Custom|SpawnNextRoom
  ;[0.15 0.15 0.15 0.5 25] Spawning the next room
  (bind _output_get (Variables|Default|SetExitPoint (.OutItem (Utilities|Array|Random (Variables|Default|GetExitsList)))))
  (bind _returnvalue (Game|SpawnActorfromClass (.OutItem (Utilities|Array|Random (Variables|Default|GetRoomList))) (Transformation|GetWorldTransform _output_get) "AlwaysSpawn" "MultiplyWithRoot" 0 0))
  (bind _asmaster_room (Utilities|Casting|CastToMaster_Room _returnvalue))
  (Variables|Default|SetLatestRoom _asmaster_room)
  (Utilities|FlowControl|Delay 0.1)
  (CallFunction|RemovingOverlaps))

(event Custom|CheckingOverlaps
  ;[0.15 0.15 0.15 0.5 25] Detect Overlapped Rooms
  (for _array_element (Components|GetChildrenComponents (Variables|/Game/Blueprints/NewStuff/Master_Room.Master_Room_C|GetOverlapFolder (Variables|Default|GetLatestRoom)) false)
    (bind _asbox_collision (Utilities|Casting|CastToBoxComponent _array_element))
    (Utilities|Array|AppendArray (Variables|Default|GetOverlapList) (Class|PrimitiveComponent|GetOverlappingComponents _asbox_collision))))

(event Custom|Removing%20Overlaps
  (bind _exitslist (Variables|Default|GetExitsList))
  ;[0.15 0.15 0.15 0.5 25] Removing Overlapping Rooms
  (CallFunction|CheckingOverlaps)
  (if (Utilities|Array|IsNotEmpty (Variables|Default|GetOverlapList))
    (Utilities|Array|Clear (Variables|Default|GetOverlapList))
    (Actor|DestroyActor (Variables|Default|GetLatestRoom))
    (CallFunction|SpawnNextRoom)
    (else
      (Utilities|Array|Clear (Variables|Default|GetOverlapList))
      (Math|Integer|DecrementInt (Variables|Default|GetRoomCount)
        (:%20%20
          (Utilities|Array|RemoveItem _exitslist (Variables|Default|GetExitPoint))
          (Utilities|Array|AppendArray _exitslist (Components|GetChildrenComponents (Variables|/Game/Blueprints/NewStuff/Master_Room.Master_Room_C|GetExitsFolder (Variables|Default|GetLatestRoom)) false))
          (if (> (Variables|Default|GetRoomCount) 0)
            (CallFunction|SpawnNextRoom)
            (else
              (CallFunction|CloseExits))))))))

(event Custom|CloseExits
  ;[0.15 0.15 0.15 0.5 25] Close Exits
  (for _array_element (Variables|Default|GetExitsList)
    (Game|SpawnActorfromClass "/Game/Blueprints/NewStuff/ExitWall.ExitWall_C" (Transformation|GetWorldTransform _array_element) "AlwaysSpawn" "MultiplyWithRoot" 0 0)))

(event EventBeginPlay
  (CallFunction|SpawnStartRoom)
  (CallFunction|SpawnNextRoom))

(fn ConstructionScript)