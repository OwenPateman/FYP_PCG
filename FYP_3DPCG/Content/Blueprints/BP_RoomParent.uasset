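; BP_RoomParent is a base room actor that opens paths to the rooms it connects to.
; On BeginPlay it caches its world XY location as Coordinates.
; CreatePaths loops over RoomConnections, compares each room's coordinates with its own, and destroys the Front, Back, Right or Left component facing that room.
; A differing X selects Front or Back; otherwise Y selects Right or Left.
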(event Custom|CreatePaths
  (bind _result (Utilities|Set|ToArray (Variables|Default|GetRoomConnections)))
  (for _array_element _result
    (if (Math|Vector|NotEqual(Vector) (Math|Conversions|ToVector2D(Vector) (.x (Variables|BP_RoomParent_C|GetCoordinates _array_element))) (Math|Conversions|ToVector2D(Vector) (.x (Variables|Default|GetCoordinates))) 0.0001)
      (if (> (.x (Variables|BP_RoomParent_C|GetCoordinates _array_element)) (.x (Variables|Default|GetCoordinates)))
        (Components|DestroyComponent (Variables|Default|GetFront))
        (else
          (Components|DestroyComponent (Variables|Default|GetBack))))
      (elif (> (.y (Variables|BP_RoomParent_C|GetCoordinates _array_element)) (.y (Variables|Default|GetCoordinates)))
        (Components|DestroyComponent (Variables|Default|GetRight))
        (else
          (Components|DestroyComponent (Variables|Default|GetLeft)))))))

(event EventBeginPlay
  (bind _returnvalue (Transformation|GetActorLocation))
  (Variables|Default|SetCoordinates (Math|Vector2D|MakeVector2D (.x _returnvalue) (.y _returnvalue))))

(fn ConstructionScript)